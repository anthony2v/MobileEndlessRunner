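; Jump power-up pickup that temporarily boosts the jump of a ThirdPersonCharacter that overlaps it.
; On actor overlap it sets the character's JumpPowerupActive flag, raises JumpZVelocity and destroys only its static mesh, keeping the actor alive for the timer.
; After a ten-second Delay it writes back a hard-coded normal velocity and clears the flag, printing a message at each change.
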(event `self.ReceiveActorBeginOverlap`
  (params (OtherActor :type "Actor Object Reference"))
  (bind _asthird_person_character (cast `/Game/ThirdPersonBP/Blueprints/ThirdPersonCharacter` OtherActor))
  (set `/Game/ThirdPersonBP/Blueprints/ThirdPersonCharacter.JumpPowerupActive` true _asthird_person_character)
  (`KismetSystemLibrary.PrintString` "JUMP BOOSTED")
  (bind _charactermovement (`Character.CharacterMovement` _asthird_person_character))
  (set `CharacterMovementComponent.JumpZVelocity` 800.0 _charactermovement)
  (`ActorComponent.K2_DestroyComponent` (`self.StaticMesh`))
  (`KismetSystemLibrary.Delay` 10.0)
  (set `CharacterMovementComponent.JumpZVelocity` 600.0 _charactermovement)
  (set `/Game/ThirdPersonBP/Blueprints/ThirdPersonCharacter.JumpPowerupActive` false _asthird_person_character)
  (`KismetSystemLibrary.PrintString` "NORMAL JUMP"))

(event `self.StaticMesh.OnComponentBeginOverlap`
  (params (OverlappedComponent :type "PrimitiveComponent Object Reference") (OtherActor :type "Actor Object Reference") (OtherComp :type "PrimitiveComponent Object Reference") (OtherBodyIndex :type Integer) (bFromSweep :type Boolean) (SweepResult :type "HitResult Structure (by ref)")))

(fn `UserConstructionScript`)